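; Kamehameha beam VFX actor that animates a growing, then thinning beam through the NSBeam effect component.
; Each Tick raises BeamHeight along Z by a fixed step and pushes it to the effect as a parameter.
; Past a height threshold, BeamWidth shrinks until it reaches zero and sets Stop, while height keeps increasing.
; Steps are per frame, unscaled by delta time, and the width prints every tick.
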(event `self.ReceiveTick`
  (params (DeltaSeconds :type "Float (single-precision)"))
  (bind _beamwidth (`self.BeamWidth`))
  (bind _output_get (set `self.BeamHeight` (+ (`self.BeamHeight`) (0.0 0.0 100.0))))
  (`FXSystemComponent.SetVectorParameter` (`self.NS_Beam`) "BeamHeight" (`self.BeamHeight`))
  (`KismetSystemLibrary.PrintString` (`KismetStringLibrary.Conv_DoubleToString` _beamwidth))
  (if (> (.z _output_get) 10000.0)
    (if (not (`self.Stop`))
      (set `self.BeamWidth` (- _beamwidth 10.0))
      (`FXSystemComponent.SetFloatParameter` (`self.NS_Beam`) "BeamWidth" (`self.BeamWidth`))
      (if (<= (`self.BeamWidth`) 0.0)
        (set `self.Stop` true)))))

(fn `UserConstructionScript`)