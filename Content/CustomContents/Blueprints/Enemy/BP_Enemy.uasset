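; Melee enemy character that targets the player on detector overlap, deals damage with kicks and reacts to being hit.
; Overlap hands the player to AIC_Enemy, while damage goes through BPCStatSystem and sets IsHit or IsDead on the Blackboard.
; Hits nudge it along the attacker's forward vector and play a random montage; death plays a montage and disables capsule collision.
; StartAttack sets a timer for a right-leg sphere trace that damages Player-tagged actors.
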(event `self.ReceiveBeginPlay`
  ; Comment
  (bind _asabp_enemy (cast `/Game/CustomContents/Blueprints/Enemy/ABP_Enemy` (`SkeletalMeshComponent.GetAnimInstance` (`self.Mesh`))))
  (set `self.AnimBP` _asabp_enemy))

(event `self.Detector.OnComponentBeginOverlap`
  (params (OverlappedComponent :type "PrimitiveComponent Object Reference") (OtherActor :type "Actor Object Reference") (OtherComp :type "PrimitiveComponent Object Reference") (OtherBodyIndex :type Integer) (bFromSweep :type Boolean) (SweepResult :type "HitResult Structure (by ref)"))
  (bind _asbp_player (cast `/Game/CustomContents/Blueprints/Player/BP_Player` OtherActor))
  (bind _asaic_enemy (cast `/Game/CustomContents/Blueprints/Enemy/AIC_Enemy` (`AIBlueprintHelperLibrary.GetAIController` self)))
  (`/Game/CustomContents/Blueprints/Enemy/AIC_Enemy.Set Target` _asaic_enemy _asbp_player))

(event `self.ReceiveAnyDamage`
  (params (Damage :type "Float (single-precision)") (DamageType :type "DamageType Object Reference") (InstigatedBy :type "Controller Object Reference") (DamageCauser :type "Actor Object Reference"))
  (bind _output_get (set `self.IsHit` true))
  (`BlackboardComponent.SetValueAsBool` (`AIBlueprintHelperLibrary.GetBlackboard` null) "IsHit" _output_get)
  (set `self.Damage Causer` DamageCauser)
  (bind _isdead (`/Game/CustomContents/Blueprints/Player/BPC_StatSystem.DecreaseHelath` (`self.BPC_StatSystem`) Damage))
  (bind _output_get_2 (set `self.Is Dead` _isdead))
  (if _output_get_2
    (`BlackboardComponent.SetValueAsBool` (`AIBlueprintHelperLibrary.GetBlackboard` null) "IsDead" (`self.Is Dead`))
    (`self.PlayAnimMontage` "/Game/CustomContents/Animation/AttackAnimations/Montage/Death_Montage.Death_Montage")
    (`PrimitiveComponent.SetCollisionEnabled` (`self.CapsuleComponent`) "NoCollision")
    (else
      (`self.SetBackEnemyLocation`)
      (bind _returnvalue (`self.PlayAnimMontage` (`self.GetRandomHitAnim`)))
      (`KismetSystemLibrary.Delay` _returnvalue)
      (bind _output_get_3 (set `self.IsHit` false))
      (`BlackboardComponent.SetValueAsBool` (`AIBlueprintHelperLibrary.GetBlackboard` null) "IsHit" _output_get_3))))

(event `StartAttack`
  (bind _returnvalue (`KismetSystemLibrary.K2_SetTimerDelegate` (delegate `Attack`) 0.01))
  (set `self.AttackTimerHandler` _returnvalue))

(event `Attack`
  (bind (_outhit _returnvalue) (`KismetSystemLibrary.SphereTraceSingle` :`Start` (`SceneComponent.K2_GetComponentLocation` (`self.RightLeg_Start`)) :`End` (`SceneComponent.K2_GetComponentLocation` (`self.RightLeg_End`)) :`Radius` 30.0 :`TraceChannel` "TraceTypeQuery1" :`DrawDebugType` "ForDuration"))
  (if _returnvalue
    (bind (_bblockinghit _binitialoverlap _time _distance _location _impactpoint _normal _impactnormal _physmat _hitactor) (`GameplayStatics.BreakHitResult` _outhit))
    (if (`self.ActorHasTag` _hitactor "Player")
      (`GameplayStatics.ApplyDamage` _hitactor 20.0 null self))))

(event `StopAttack`
  (`KismetSystemLibrary.K2_ClearAndInvalidateTimerHandle` (`self.AttackTimerHandler`)))

(fn `GetRandomHitAnim`
  (returns (Output :type "AnimMontage Object Reference"))
  (return (`|GetArrayItem` (`self.HitMontages`) (`KismetMathLibrary.RandomIntegerInRange` 0 (- (`KismetArrayLibrary.Array_Length` (`self.HitMontages`)) 1)))))

(fn `SetBackEnemyLocation`
  (`self.K2_SetActorLocation` (+ (* (`self.GetActorForwardVector` (`self.Damage Causer`)) 20.0) (`self.K2_GetActorLocation`))))

(fn `UserConstructionScript`)