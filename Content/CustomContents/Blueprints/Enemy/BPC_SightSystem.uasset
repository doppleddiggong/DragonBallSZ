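; Enemy sight component that detects when a target set through InitSight enters its owner's view cone.
; Each Tick checks distance and forward-vector angle, calling SightDetectTarget only when detection state changes.
; Time since that change accumulates, and LerpAlpha exposes it as a clamped 0–1 ratio of Duration.
; The cone and line traces only draw debug visuals; trace results are unused, so obstacles never block detection.
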(event `InitSight`
  (params (Target :type "Actor Object Reference") (SightLength :type "Float (double-precision)") (SightAngle :type "Float (double-precision)"))
  (set `self.TargetActor` Target)
  (set `self.SightLength` SightLength)
  (set `self.SightAngle` SightAngle))

(event `self.ReceiveBeginPlay`
  (set `self.OwnerActor` (`self.GetOwner`)))

(event `self.ReceiveTick`
  (params (DeltaSeconds :type "Float (single-precision)"))
  (if (and (`KismetSystemLibrary.IsValid` (`self.OwnerActor`)) (`KismetSystemLibrary.IsValid` (`self.TargetActor`)))
    (`|ExecutionSequence`
      (:`then_0`
        (`self.SightLineTrace` (`self.SightLength`) (`self.SightAngle`)))
      (:`then_1`
        ; Sight Process
        (if (and (`self.DetectSightLegnth` (`self.SightLength`)) (`self.DetectSightAngle` (`self.SightAngle`))) :!pinned true
          (if (`self.DetectTarget`)
            (`self.AddElapsedTime`)
            (`KismetSystemLibrary.PrintString` "Detect Target1")
            (else
              (set `self.DetectTarget` true)
              (set `self.ElapsedTime` 0.0)
              (`KismetSystemLibrary.PrintString` "Detect Target2")
              (`self.SightDetectTarget` (`self.DetectTarget`))))
          (elif (`self.DetectTarget`)
            (set `self.DetectTarget` false)
            (set `self.ElapsedTime` 0.0)
            (`KismetSystemLibrary.PrintString` "Missing Target1")
            (`self.SightDetectTarget` (`self.DetectTarget`))
            (else
              (`self.AddElapsedTime`)
              (`KismetSystemLibrary.PrintString` "Missing Target2"))))))))

(fn `AddElapsedTime`
  (set `self.ElapsedTime` (+ (`self.ElapsedTime`) (`GameplayStatics.GetWorldDeltaSeconds`))))

(fn `DetectSightAngle`
  (params (SAngle :type "Float (double-precision)"))
  (returns (ReturnValue :type Boolean))
  (bind _returnvalue (`KismetMathLibrary.DegAcos` (`KismetMathLibrary.Dot_VectorVector` (`Actor.GetActorForwardVector` (`self.OwnerActor`)) (`KismetMathLibrary.Normal` (- (`Actor.K2_GetActorLocation` (`self.TargetActor`)) (`Actor.K2_GetActorLocation` (`self.OwnerActor`)))))))
  (return (and (>= _returnvalue 0.0) (<= _returnvalue SAngle))))

(fn `DetectSightLegnth`
  (params (SLength :type "Float (double-precision)"))
  (returns (ReturnValue :type Boolean))
  (return (< (`KismetMathLibrary.Vector_Distance` (`Actor.K2_GetActorLocation` (`self.TargetActor`)) (`Actor.K2_GetActorLocation` (`self.OwnerActor`))) SLength)))

(fn `LerpAlpha`
  (returns (ReturnValue :type "Float (double-precision)"))
  (return (`KismetMathLibrary.FClamp` (/ (`self.ElapsedTime`) (`self.Duration`)))))

(fn `SightLineTrace`
  (params (Length :type "Float (double-precision)") (Angle :type "Float (double-precision)"))
  (locals (SLength :type "Float (double-precision)") (SAngle :type "Float (double-precision)"))
  (set `local.SLength` Length)
  (set `local.SAngle` Angle)
  (`KismetSystemLibrary.DrawDebugConeInDegrees` (`Actor.K2_GetActorLocation` (`self.OwnerActor`)) (`Actor.GetActorForwardVector` (`self.OwnerActor`)) (`local.Length`) (`local.Angle`) 1.0 12 (struct :`R` 1.0 :`B` 0.149419 :`A` 1.0))
  (if (`self.DetectTarget`)
    ; Line1
    (`KismetSystemLibrary.LineTraceSingle` :`Start` (`Actor.K2_GetActorLocation` (`self.OwnerActor`)) :`End` (+ (`Actor.K2_GetActorLocation` (`self.OwnerActor`)) (* (`KismetMathLibrary.GetForwardVector` (`Actor.K2_GetActorRotation` (`self.OwnerActor`))) (`local.Length`))) :`TraceChannel` "TraceTypeQuery1" :`DrawDebugType` "ForDuration" :`TraceColor` (struct :`R` 0.921582 :`G` 0.768151 :`A` 1.0) :`DrawTime` 0.0)
    ; Line2
    (`KismetSystemLibrary.LineTraceSingle` :`Start` (`Actor.K2_GetActorLocation` (`self.OwnerActor`)) :`End` (+ (`Actor.K2_GetActorLocation` (`self.OwnerActor`)) (* (`KismetMathLibrary.GreaterGreater_VectorRotator` (`KismetMathLibrary.GetForwardVector` (`Actor.K2_GetActorRotation` (`self.OwnerActor`))) (`KismetMathLibrary.MakeRotator` 0.0 0.0 (* (`local.Angle`) -1.0))) (`local.Length`))) :`TraceChannel` "TraceTypeQuery1" :`DrawDebugType` "ForDuration" :`TraceColor` (struct :`R` 0.921582 :`G` 0.768151 :`A` 1.0) :`DrawTime` 0.0)
    ; Line3
    (`KismetSystemLibrary.LineTraceSingle` :`Start` (`Actor.K2_GetActorLocation` (`self.OwnerActor`)) :`End` (+ (`Actor.K2_GetActorLocation` (`self.OwnerActor`)) (* (`KismetMathLibrary.GreaterGreater_VectorRotator` (`KismetMathLibrary.GetForwardVector` (`Actor.K2_GetActorRotation` (`self.OwnerActor`))) (`KismetMathLibrary.MakeRotator` 0.0 0.0 (`local.Angle`))) (`local.Length`))) :`TraceChannel` "TraceTypeQuery1" :`DrawDebugType` "ForDuration" :`TraceColor` (struct :`R` 0.921582 :`G` 0.768151 :`A` 1.0) :`DrawTime` 0.0)))