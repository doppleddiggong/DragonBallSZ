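; Player component that runs a four-hit melee punch combo (jab, straight, two hooks) from the attack input.
; Each press plays the montage for the current combo count at a shared attack speed, blocked while an attack is active.
; A montage notify reopens input and advances or wraps the count, while a timer started with each hit resets it to the first attack.
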(event `self.ReceiveBeginPlay`
  ; Comment
  (bind _asbp_player (cast `/Game/CustomContents/Blueprints/Player/BP_Player` (`self.GetOwner`)))
  (bind _output_get (set `self.Player` _asbp_player))
  (set `self.Mesh` (`Character.Mesh` _output_get)))

(event `EnhancedInput|/Game/CustomContents/Input/IA_DBSZ_Attack`
  (params (ActionValue :type Boolean) (ElapsedSeconds :type "Float (double-precision)") (TriggeredSeconds :type "Float (double-precision)") (InputAction :type "InputAction Object Reference" :default "/Game/CustomContents/Input/IA_DBSZ_Attack.IA_DBSZ_Attack"))
  (:`Started`
    (if (not (`self.IsAttacking`))
      (set `self.IsAttacking` true)
      (switch `int` (`self.ComboCount`)
        (:`0`
          (`|PlayMontage` (`self.Mesh`) "/Game/CustomContents/Animation/AttackAnimations/Montage/Attack1_Jab_Montage.Attack1_Jab_Montage" (`self.AttackSpeed`)
            (:`then`
              (`KismetSystemLibrary.PrintString` "Atk1")
              (`KismetSystemLibrary.K2_SetTimerDelegate` (delegate `ResetCounter`) 3.0 :!label _label))
            (:`OnNotifyBegin`
              (set `self.IsAttacking` false)
              (set `self.ComboCount` 1))))
        (:`1`
          (`|PlayMontage` (`self.Mesh`) "/Game/CustomContents/Animation/AttackAnimations/Montage/Attack2_Straight_Montage.Attack2_Straight_Montage" (`self.AttackSpeed`)
            (:`then`
              (`KismetSystemLibrary.PrintString` "Atk2")
              (goto _label))
            (:`OnNotifyBegin`
              (set `self.IsAttacking` false)
              (set `self.ComboCount` 2))))
        (:`2`
          (`|PlayMontage` (`self.Mesh`) "/Game/CustomContents/Animation/AttackAnimations/Montage/Attack3_Hook_Montage.Attack3_Hook_Montage" (`self.AttackSpeed`)
            (:`then`
              (`KismetSystemLibrary.PrintString` "Atk3")
              (goto _label))
            (:`OnNotifyBegin`
              (set `self.IsAttacking` false)
              (set `self.ComboCount` 3))))
        (:`3`
          (`|PlayMontage` (`self.Mesh`) "/Game/CustomContents/Animation/AttackAnimations/Montage/Attack4_Hook_Montage.Attack4_Hook_Montage" (`self.AttackSpeed`)
            (:`then`
              (`KismetSystemLibrary.PrintString` "Atk4")
              (goto _label))
            (:`OnNotifyBegin`
              (set `self.IsAttacking` false)
              (set `self.ComboCount` 0))))))))

(event `ResetCounter`
  (set `self.ComboCount` 0))