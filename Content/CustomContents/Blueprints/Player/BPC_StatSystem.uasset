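; Player stat component that tracks current health against a maximum and holds a death flag.
; On BeginPlay, InitStat fills health to the maximum and clears the flag.
; IncreaseHealth adds health capped at the maximum, without checking or clearing the death flag.
; DecreaseHelath subtracts damage, and when health drops below zero it clamps to zero, sets the flag and returns it.
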(event `self.ReceiveBeginPlay`
  (`self.InitStat`))

(fn `DecreaseHelath`
  (params (DamagePoint :type "Float (double-precision)"))
  (returns (IsDead :type Boolean))
  (bind _output_get (set `self.CurHP` (- (`self.CurHP`) DamagePoint)))
  (if (< _output_get 0.0)
    (set `self.CurHP` 0.0)
    (bind _output_get_2 (set `self.IsDead` true))
    (return _output_get_2)))

(fn `IncreaseHealth`
  (params (Value :type "Float (double-precision)"))
  (set `self.CurHP` (+ Value (`self.CurHP`)))
  (if (> (`self.CurHP`) (`self.MaxHP`))
    (set `self.CurHP` (`self.MaxHP`))))

(fn `InitStat`
  (set `self.CurHP` (`self.MaxHP`))
  (set `self.IsDead` false))