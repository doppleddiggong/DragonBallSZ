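; Player character Blueprint that hands the view to the level's BP_DynamicCamera on BeginPlay and calls SetHold(false) every Tick.
; Its move command and AnyDamage events are empty, leaving the movement and damage logic disconnected.
; That unwired logic moves along actor axes by movement mode, and decreases health through StatSystem, playing a death montage or knockback with a random hit animation.
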(event `self.ReceiveBeginPlay`
  ; Comment
  (bind _returnvalue (`GameplayStatics.GetActorOfClass` "/Game/DynamicCamera/BP_DynamicCamera.BP_DynamicCamera_C"))
  (`PlayerController.SetViewTargetWithBlend` (`GameplayStatics.GetPlayerController` 0) _returnvalue 0.0 "VTBlend_Linear" 0.0 false))

(event `self.ReceiveAnyDamage`
  (params (Damage :type "Float (single-precision)") (DamageType :type "DamageType Object Reference") (InstigatedBy :type "Controller Object Reference") (DamageCauser :type "Actor Object Reference"))
  ; Comment
)

(event `self.ReceiveTick`
  (params (DeltaSeconds :type "Float (single-precision)"))
  (`self.SetHold` false))

(event `Cmd_Move_1`
  (params (Axis :type "Vector2D Structure (by ref)") (Axis_X :type "Float (double-precision)") (Axis_Y :type "Float (double-precision)"))
  ; Comment
)

(fn `GetRandomHitAnim2`)

(fn `SetKnockbackLocation`
  (params (DamageCauser :type "Actor Object Reference"))
  (`self.K2_SetActorLocation` (+ (* (`self.GetActorForwardVector` DamageCauser) 20.0) (`self.K2_GetActorLocation`))))

(fn `UserConstructionScript`)