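; Player melee component that runs a four-punch montage combo (jab, straight, two hooks) from the attack input on BP_Player.
; Montage notifies unlock and advance the combo; a timer resets it, as does an interruption by a hit.
; StartAttackTrace and StopAttackTrace set and clear a timer for a debug-drawn sphere trace from the left or right hand, chosen by combo index, that applies damage.
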(event `EnhancedInput|/Game/CustomContents/Input/IA_DBSZ_Attack`
  (params (ActionValue :type Boolean) (ElapsedSeconds :type "Float (double-precision)") (TriggeredSeconds :type "Float (double-precision)") (InputAction :type "InputAction Object Reference" :default "/Game/CustomContents/Input/IA_DBSZ_Attack.IA_DBSZ_Attack"))
  ; Comment
  (:`Started`
    (if (and (not (`/Game/CustomContents/Blueprints/Character/Player/BP_Player.IsHit` (`self.Player`))) (not (`self.IsAttacking`)))
      (set `self.IsAttacking` true)
      (switch `int` (`self.ComboCount`)
        (:`0`
          (`|PlayMontage` (`self.Mesh`) "/Game/CustomContents/Animation/AttackAnimations/Montage/Attack1_Jab_Montage.Attack1_Jab_Montage" (`self.AttackSpeed`)
            (:`then`
              (`KismetSystemLibrary.PrintString` "Atk1")
              (`KismetSystemLibrary.K2_SetTimerDelegate` (delegate `ResetCounter`) 3.0 :!label _label))
            (:`OnInterrupted`
              (`self.ResetByHit`))
            (:`OnNotifyBegin`
              (set `self.IsAttacking` false)
              (set `self.ComboCount` 1))))
        (:`1`
          (`|PlayMontage` (`self.Mesh`) "/Game/CustomContents/Animation/AttackAnimations/Montage/Attack2_Straight_Montage.Attack2_Straight_Montage" (`self.AttackSpeed`)
            (:`then`
              (`KismetSystemLibrary.PrintString` "Atk2")
              (goto _label))
            (:`OnInterrupted`
              (`self.ResetByHit`))
            (:`OnNotifyBegin`
              (set `self.IsAttacking` false)
              (set `self.ComboCount` 2))))
        (:`2`
          (`|PlayMontage` (`self.Mesh`) "/Game/CustomContents/Animation/AttackAnimations/Montage/Attack3_Hook_Montage.Attack3_Hook_Montage" (`self.AttackSpeed`)
            (:`then`
              (`KismetSystemLibrary.PrintString` "Atk3")
              (goto _label))
            (:`OnInterrupted`
              (`self.ResetByHit`))
            (:`OnNotifyBegin`
              (set `self.IsAttacking` false)
              (set `self.ComboCount` 3))))
        (:`3`
          (`|PlayMontage` (`self.Mesh`) "/Game/CustomContents/Animation/AttackAnimations/Montage/Attack4_Hook_Montage.Attack4_Hook_Montage" (`self.AttackSpeed`)
            (:`then`
              (`KismetSystemLibrary.PrintString` "Atk4")
              (goto _label))
            (:`OnInterrupted`
              (`self.ResetByHit`))
            (:`OnNotifyBegin`
              (set `self.IsAttacking` false)
              (set `self.ComboCount` 0))))))))

(event `ResetCounter`
  ; Comment
  (set `self.ComboCount` 0))

(event `StopAttackTrace`
  ; Comment
  (`KismetSystemLibrary.K2_ClearAndInvalidateTimerHandle` (`self.AttackTimerHandler`)))

(event `ResetByHit`
  (if (`/Game/CustomContents/Blueprints/Character/Player/BP_Player.IsHit` (`self.Player`))
    (set `self.IsAttacking` false)
    (set `self.ComboCount` 0)))

(event `self.ReceiveBeginPlay`
  ; Comment
  (bind _asbp_player (cast `/Game/CustomContents/Blueprints/Character/Player/BP_Player` (`self.GetOwner`)))
  (bind _output_get (set `self.Player` _asbp_player))
  (set `self.Mesh` (`Character.Mesh` _output_get)))

(event `StartAttackTrace`
  ; Comment
  (bind _returnvalue (`KismetSystemLibrary.K2_SetTimerDelegate` (delegate `AttackTrace`) 0.01))
  (set `self.AttackTimerHandler` _returnvalue))

(event `AttackTrace`
  (bind (_start _end) (`self.GetHandLocation` (`/Game/CustomContents/Blueprints/Character/Player/BP_Player.RightHand` (`self.Player`))))
  (bind (_start_2 _end_2) (`self.GetHandLocation` (`/Game/CustomContents/Blueprints/Character/Player/BP_Player.LeftHand` (`self.Player`))))
  ; Comment
  (switch `int` (`self.ComboCount`)
    (:`0`
      (`self.AttackSphereTrace` _start_2 _end_2 (`self.Damage`) (`self.Player`) :!label _label_2))
    (:`1`
      (`self.AttackSphereTrace` _start _end (`self.Damage`) (`self.Player`) :!label _label_3))
    (:`2`
      (goto _label_2))
    (:`3`
      (goto _label_3))))

(fn `AttackSphereTrace`
  (params (Start :type "Vector Structure") (End :type "Vector Structure") (BaseDamage :type "Float (single-precision)") (DamageCauser :type "Actor Object Reference"))
  (bind (_outhit _returnvalue) (`KismetSystemLibrary.SphereTraceSingle` :`Start` Start :`End` End :`Radius` 20.0 :`TraceChannel` "TraceTypeQuery1" :`DrawDebugType` "ForDuration" :`DrawTime` 7.0))
  (if _returnvalue
    (`GameplayStatics.ApplyDamage` (`.HitActor` (`GameplayStatics.BreakHitResult` _outhit)) BaseDamage null DamageCauser)))

(fn `GetHandLocation`
  (params (Hand :type "SceneComponent Object Reference"))
  (returns (Start :type "Vector Structure") (End :type "Vector Structure"))
  (return (`SceneComponent.K2_GetComponentLocation` Hand) (`KismetMathLibrary.TransformLocation` (`SceneComponent.K2_GetComponentToWorld` Hand) (+ (`SceneComponent.RelativeLocation` Hand) (20.0 0.0 0.0)))))