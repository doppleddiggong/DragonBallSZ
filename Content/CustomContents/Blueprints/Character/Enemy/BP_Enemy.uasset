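; BP_Enemy is an enemy character that takes damage, reacts to hits, dies and attacks through a RushAttackSystem.
; AnyDamage feeds StatSystem.DecreaseHealth, then either plays a death montage and disables capsule collision, or nudges the enemy along the damage causer's forward vector with a random hit montage.
; IsHit and IsDead are mirrored to the Blackboard, with IsHit cleared after the montage's duration.
; StartAttack and StopAttack set and clear a short timer that calls OnAttack.
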(event `self.ReceiveAnyDamage`
  (params (Damage :type "Float (single-precision)") (DamageType :type "DamageType Object Reference") (InstigatedBy :type "Controller Object Reference") (DamageCauser :type "Actor Object Reference"))
  ; Comment
  (set `self.Damage Causer` DamageCauser)
  (bind _output_get (set `self.IsHit` true))
  (`BlackboardComponent.SetValueAsBool` (`AIBlueprintHelperLibrary.GetBlackboard` null) "IsHit" _output_get)
  (bind _returnvalue (`StatSystem.DecreaseHealth` (`self.StatSystem`) Damage))
  (if _returnvalue
    ; Comment
    (`BlackboardComponent.SetValueAsBool` (`AIBlueprintHelperLibrary.GetBlackboard` null) "IsDead" true)
    (`self.PlayAnimMontage` "/Game/CustomContents/Animation/AttackAnimations/Montage/Death_Montage.Death_Montage")
    (`PrimitiveComponent.SetCollisionEnabled` (`self.CapsuleComponent`) "NoCollision")
    (else
      ; Comment
      (`self.SetKnockbackLocation` (`self.Damage Causer`))
      (bind _returnvalue_2 (`self.PlayAnimMontage` (`self.GetRandomHitAnim`)))
      (`KismetSystemLibrary.Delay` _returnvalue_2)
      (bind _output_get_2 (set `self.IsHit` false))
      (`BlackboardComponent.SetValueAsBool` (`AIBlueprintHelperLibrary.GetBlackboard` null) "IsHit" _output_get_2))))

(event `StartAttack`
  ; Comment
  (bind _returnvalue (`KismetSystemLibrary.K2_SetTimerDelegate` (delegate `Attack`) 0.01))
  (set `self.AttackTimerHandler` _returnvalue))

(event `Attack`
  ; Comment
  (`RushAttackSystem.OnAttack` (`self.RushAttackSystem`)))

(event `StopAttack`
  ; Comment
  (`KismetSystemLibrary.K2_ClearAndInvalidateTimerHandle` (`self.AttackTimerHandler`)))

(fn `GetRandomHitAnim`
  (returns (Output :type "AnimMontage Object Reference"))
  (return (`|GetArrayItem` (`self.HitMontages`) (`KismetMathLibrary.RandomIntegerInRange` 0 (- (`KismetArrayLibrary.Array_Length` (`self.HitMontages`)) 1)))))

(fn `SetKnockbackLocation`
  (params (DamageCauser :type "Actor Object Reference"))
  (`self.K2_SetActorLocation` (+ (* (`self.GetActorForwardVector` DamageCauser) 20.0) (`self.K2_GetActorLocation`))))

(fn `UserConstructionScript`)