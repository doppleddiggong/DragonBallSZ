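; BP_DynamicCamera is a lock-on camera prototype meant to frame BP_Player and BP_Enemy, but its BeginPlay and Tick are empty and the main logic is disconnected.
; PlayerROT yaws the player toward the target, and ResetCameraRotation, despite its name, eases the camera position behind the player, opposite the target.
; Unwired chains fetch both actors and use screen-space dead zones to interpolate camera position and aim at their midpoint.
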(event `self.ReceiveBeginPlay`)

(event `self.ReceiveTick`
  (params (DeltaSeconds :type "Float (single-precision)")))

(event `PlayerROT`
  ; 락온 중 플레이어 회전 잠금
  (`self.K2_SetActorRotation` (`self.PlayerRef`) (`KismetMathLibrary.MakeRotator` (.roll (`self.K2_GetActorRotation` (`self.PlayerRef`))) (.pitch (`self.K2_GetActorRotation` (`self.PlayerRef`))) (.yaw (`KismetMathLibrary.FindLookAtRotation` (`self.K2_GetActorLocation` (`self.PlayerRef`)) (`self.K2_GetActorLocation` (`self.TargetRef`))))) false))

(event `Reset Camera Rotation`
  (`self.K2_SetActorLocation` (`KismetMathLibrary.VInterpTo` (`self.K2_GetActorLocation`) (+ (`self.K2_GetActorLocation` (`self.PlayerRef`)) (* (`KismetMathLibrary.Normal` (- (`self.K2_GetActorLocation` (`self.PlayerRef`)) (`self.K2_GetActorLocation` (`self.TargetRef`)))) 300.0) (0.0 0.0 100.0)) (`GameplayStatics.GetWorldDeltaSeconds`) 2.0)))

(fn `UserConstructionScript`)